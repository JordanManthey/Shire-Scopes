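; Game instance that manages online sessions through the AdvancedSessions plugin: hosting, finding, joining and ending them.
; An IsMatchmaking flag, stored as a byte because Steam search cannot filter bools, tags hosted sessions and filters search results in a separate node, since the built-in filter fails.
; Changing public or invite-only status destroys and re-hosts the session.
; Accepted invites join behind a loading screen, returning to MainMenu on failure.
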(event `Find Sessions`
  (params (bIsMatchmaking :type Boolean))
  (`self.SetFindSessionFilters` bIsMatchmaking)
  (bind _results (`FindSessionsCallbackProxyAdvanced.FindSessionsAdvanced` (`GameplayStatics.GetPlayerController` 0) 100 (`self.Debug_bUseLAN`) "AllServers") ; Filter param does not work. Use independent filter node.
    (:`OnSuccess`
      (bind _filteredresults (`FindSessionsCallbackProxyAdvanced.FilterSessionResults` _results (`self.FindSessionFilters`)))
      (`self.OnSessionsFound` _filteredresults))))

(event `Set Session Type`
  (params (bIsPublic :type Boolean))
  ;[1 1 1] Used when a Lobby Host updates the session to be Public or InviteOnly
  (`DestroySessionCallbackProxy.DestroySession` (`GameplayStatics.GetPlayerController` 0)
    (:`OnSuccess`
      (`self.OnSessionReadyUpdate` false)
      (`self.Host Session` bIsPublic))))

(event `End Session`
  (`DestroySessionCallbackProxy.DestroySession` (`GameplayStatics.GetPlayerController` 0)
    (:`OnSuccess`
      (`self.OnSessionReadyUpdate` false))))

(event `Host Session`
  (params (bIsPublic :type Boolean) (bIsMatchmaking :type Boolean))
  (`self.SetCreateSessionProperties` bIsMatchmaking)
  (bind _ascustom_game_mode (cast `CustomGameMode` (`GameplayStatics.GetGameMode`)))
  (`CreateSessionCallbackProxyAdvanced.CreateAdvancedSession` (`self.CreateSessionProperties`) (`GameplayStatics.GetPlayerController` 0) (`CustomGameMode.MaxPlayers` _ascustom_game_mode) 100 (`self.Debug_bUseLAN`) true false true true true false false false bIsPublic
    (:`OnSuccess`
      (`self.OnSessionReadyUpdate` true))))

(event `self.EndClientSession`
  (params (Player :type "PlayerController Object Reference"))
  (`DestroySessionCallbackProxy.DestroySession` Player
    (:`OnSuccess`
      (`self.OnSessionReadyUpdate` false))))

(event `self.OnSessionInviteAccepted`
  (params (LocalPlayerNum :type Integer) (PersonInvited :type "BPUniqueNetId Structure") (SessionToJoin :type "BlueprintSessionResult Structure (by ref)"))
  (`self.Join Session` SessionToJoin))

(event `self.OnSessionInviteReceived`
  (params (LocalPlayerNum :type Integer) (PersonInviting :type "BPUniqueNetId Structure") (AppId :type String) (SessionToJoin :type "BlueprintSessionResult Structure (by ref)"))
  ;[1 1 1 1 14] This is broken in the AdvancedSessions plugin.
)

(event `Join Session`
  (params (Session :type "BlueprintSessionResult Structure"))
  (bind _returnvalue (`GameplayStatics.GetPlayerController` 0))
  (`self.CacheGameStateClass`)
  (bind _ascustom_player_controller (cast `CustomPlayerController` _returnvalue))
  (`CustomPlayerController.Client_ToggleLoadingScreen` _ascustom_player_controller true "Joining Lobby")
  (`JoinSessionCallbackProxy.JoinSession` _returnvalue Session
    (:`OnFailure`
      (bind _ascustom_player_controller_2 (cast `CustomPlayerController` (`GameplayStatics.GetPlayerController` 0)))
      (`CustomPlayerController.Client_TravelToLevel` _ascustom_player_controller_2 "MainMenu" "Failed to Join" "gameMessage=joinfail"))))