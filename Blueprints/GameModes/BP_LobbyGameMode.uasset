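; Lobby game mode that manages the hosted session from lobby creation to game start or closure.
; On BeginPlay it has BP_ShireGameInstance host a private, non-matchmaking session.
; Starting the game ends that session and launches the chosen map, passing the game mode by its class display name.
; Closing the lobby ends the session and travels to MainMenu with a "hostless" game message in the URL options.
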(event `self.ReceiveBeginPlay`
  (bind _asbp_shire_game_instance (cast `/Game/Blueprints/State/BP_ShireGameInstance` (`GameplayStatics.GetGameInstance`)))
  (`/Game/Blueprints/State/BP_ShireGameInstance.Host Session` _asbp_shire_game_instance false false))

(event `On Start Game`
  (params (`Map Name` :type String) (`Game Mode` :type "GameModeBase Class Reference"))
  (bind _asbp_shire_game_instance (cast `/Game/Blueprints/State/BP_ShireGameInstance` (`GameplayStatics.GetGameInstance`)))
  (`/Game/Blueprints/State/BP_ShireGameInstance.End Session` _asbp_shire_game_instance)
  (`self.StartGame` `Map Name` (`KismetSystemLibrary.GetClassDisplayName` `Game Mode`)))

(event `On Close Lobby`
  (bind _asbp_shire_game_instance (cast `/Game/Blueprints/State/BP_ShireGameInstance` (`GameplayStatics.GetGameInstance`)))
  (`/Game/Blueprints/State/BP_ShireGameInstance.End Session` _asbp_shire_game_instance)
  (`self.TravelToLevel` "MainMenu" false "" "?gameMessage=hostless"))

(fn `UserConstructionScript`)