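; Matchmaking game mode that automatically places the player into a public session and starts matches on random levels.
; On BeginPlay it searches through BP_ShireGameInstance, joining the lowest-ping session found or hosting a public matchmaking session if none exist.
; Starting the game ends the session and loads a level picked randomly from DT_Levels.
; Returning to menu ends the session and client-travels to MainMenu.
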(event `self.ReceiveBeginPlay`
  (bind _asbp_shire_game_instance (cast `/Game/Blueprints/State/BP_ShireGameInstance` (`GameplayStatics.GetGameInstance`)))
  (bind _output_get (set `self.Shire Game Instance` _asbp_shire_game_instance))
  (add `/Game/Blueprints/State/BP_ShireGameInstance.OnSessionsFound` _output_get (`|CreateDelegate` :!event `On Sessions Found`))
  (`/Game/Blueprints/State/BP_ShireGameInstance.Find Sessions` (`self.Shire Game Instance`) true))

(event `On Sessions Found`
  (params (`Session Results` :type "Array of BlueprintSessionResult Structure"))
  (if (`KismetArrayLibrary.Array_IsNotEmpty` `Session Results`)
    (bind _target_session (`self.GetOptimalSession` `Session Results`))
    (`/Game/Blueprints/State/BP_ShireGameInstance.Join Session` (`self.Shire Game Instance`) _target_session)
    (else
      (`/Game/Blueprints/State/BP_ShireGameInstance.Host Session` (`self.Shire Game Instance`) true true))))

(event `Return To Menu`
  (bind _asbp_shire_game_instance (cast `/Game/Blueprints/State/BP_ShireGameInstance` (`GameplayStatics.GetGameInstance`)))
  (`/Game/Blueprints/State/BP_ShireGameInstance.End Session` _asbp_shire_game_instance)
  (bind _ascustom_player_controller (cast `CustomPlayerController` (`GameplayStatics.GetPlayerController` 0)))
  (`CustomPlayerController.Client_TravelToLevel` _ascustom_player_controller "MainMenu" "Returning To Menu" ""))

(event `self.OnStartGame`
  (bind _asbp_shire_game_instance (cast `/Game/Blueprints/State/BP_ShireGameInstance` (`GameplayStatics.GetGameInstance`)))
  (`/Game/Blueprints/State/BP_ShireGameInstance.End Session` _asbp_shire_game_instance)
  (`self.StartGame` (`self.GetRandomLevelName`)))

(fn `GetOptimalSession`
  (params (`Session Results` :type "Array of BlueprintSessionResult Structure"))
  (returns (`Target Session` :type "BlueprintSessionResult Structure"))
  (locals (MinPing :type Integer) (MinPingSession :type "BlueprintSessionResult Structure"))
  (for _array_element `Session Results`
    (if (`AdvancedSessionsLibrary.IsValidSession` (`local.MinPingSession`))
      (bind _returnvalue (`FindSessionsCallbackProxy.GetPingInMs` _array_element))
      (if (< _returnvalue (`local.MinPing`))
        (set `local.MinPingSession` _array_element :!label _label)
        (set `local.MinPing` _returnvalue))
      (else
        (goto _label))))
  (return (`local.MinPingSession`)))

(fn `GetRandomLevelName`
  (returns (ReturnValue :type String))
  (bind _outrownames (`DataTableFunctionLibrary.GetDataTableRowNames` "/Game/Data/DT_Levels.DT_Levels"))
  (bind _returnvalue (`|GetDataTableRow` "/Game/Data/DT_Levels.DT_Levels" (`|GetArrayItem` _outrownames (`KismetMathLibrary.RandomInteger` (`KismetArrayLibrary.Array_Length` _outrownames))))
    (:`then`
      (return (`.LevelName_7_F8309EF74D68EF58D02D349EA06CA555` (break `/Game/Data/F_LevelData` _returnvalue))))))

(fn `UserConstructionScript`)