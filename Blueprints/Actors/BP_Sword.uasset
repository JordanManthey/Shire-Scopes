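; BP_Sword is a sword actor that plays a swing sound when activated.
; On BeginPlay it binds a handler to OnActivate, which plays the sound only if the owning character is a locally controlled player.
; PlayRandomSwingSound picks one of two swing sounds and plays it at a location with randomized pitch for variation.
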(event `self.ReceiveBeginPlay`
  (add `self.OnActivate` (`|CreateDelegate` :!event `On Activate`)))

(event `On Activate`
  (bind _owningcharacter (`self.OwningCharacter`))
  (if (and (`Pawn.IsPlayerControlled` _owningcharacter) (`Pawn.IsLocallyControlled` _owningcharacter))
    (`self.Play Random Swing Sound`)))

(fn `Play Random Swing Sound`
  (locals (`Swing Sound` :type "SoundBase Object Reference"))
  (if (`KismetMathLibrary.RandomBool`)
    (set `local.Swing Sound` "/Game/Audio/Weapons/SwordSwing1.SwordSwing1")
    (else
      (set `local.Swing Sound` "/Game/Audio/Weapons/SwordSwing2.SwordSwing2")))
  (`GameplayStatics.PlaySoundAtLocation` (`local.Swing Sound`) (0.0 0.0 0.0) (struct) 0.75 (`KismetMathLibrary.RandomFloatInRange` 0.8 1.2) 0.0 null null null null))

(fn `UserConstructionScript`)