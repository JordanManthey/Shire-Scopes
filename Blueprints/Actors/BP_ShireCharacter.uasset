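; Shire player character Blueprint that handles the HUD hookup, weapon feel, mesh selection and sound effects.
; Base character and ranged weapon events drive recoil and ADS timelines, with firing restarting recoil and reversing ADS, plus muzzle flash and movement, equip and death sounds.
; Mesh setup async-loads random first- and third-person meshes, choosing third-person pool and anim class by team relative to the local player.
; Jump and equip sounds play 2D for the local player, spatialized otherwise.
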(event `self.ReceiveBeginPlay`
  ;[1 1 1] Setup
  (bind _aswbp_player_hud (cast `/Game/Blueprints/UI/HUD/WBP_PlayerHUD` (`self.HUD`))
    (:`then`
      (`/Game/Blueprints/UI/HUD/WBP_PlayerHUD.Bind To Weapon Events` _aswbp_player_hud))
    (:`CastFailed`
      _))
  (`self.Bind To Base Events`)
  (`self.Setup Recoil Timeline`)
  (`self.Setup ADS Timeline`))

(event `self.SetupCharacterMesh`
  ;[1 1 1] Setup
  (`self.Choose Character Mesh`))

(event `On HUD Ready`
  ;[1 1 1] HUD
  (bind _aswbp_player_hud (cast `/Game/Blueprints/UI/HUD/WBP_PlayerHUD` (`self.HUD`)))
  (`/Game/Blueprints/UI/HUD/WBP_PlayerHUD.Bind To Character Events` _aswbp_player_hud)
  (`/Game/Blueprints/UI/HUD/WBP_PlayerHUD.Bind To Weapon Events` _aswbp_player_hud))

(event `On Ranged Weapon Activate`
  ;[1 1 1] Ranged Weapon
  (`|ExecutionSequence`
    (:`then_0`
      (bind (_direction _recoil_alpha_track) (`Timeline|Recoil Timeline` :!via `PlayFromStart`)
        (:`Update`
          (`self.ApplyWeaponRecoil` _recoil_alpha_track))))
    (:`then_1`
      (bind (_direction_2 _ads) (`Timeline|ADS Timeline` :!via `Reverse` :!label _label)
        (:`Update`
          (`self.ApplyWeaponAimEffects` _ads))
        (:`Finished`
          (`self.ADS Finished`))))))

(event `On Death`
  (params (`Death Character` :type "ShireCharacter Object Reference"))
  ;[1 1 1] SFX
  (`self.Play Random Death Sound`))

(event `On Land`
  ;[1 1 1] SFX
  (`GameplayStatics.PlaySoundAtLocation` "/Game/Audio/Movement/Land1.Land1" (`self.K2_GetActorLocation`) (struct) 0.5 (`KismetMathLibrary.RandomFloatInRange` 0.9 1.1) 0.0 "/Game/Audio/Movement/ATT_FootstepSound.ATT_FootstepSound" null null null))

(event `On Aim`
  ;[1 1 1] Ranged Weapon
  (goto _label))

(event `On Aim Release`
  ;[1 1 1] Ranged Weapon
  (goto _label :!via `Reverse`))

(event `On Slide Jump`
  ;[1 1 1] SFX
  (`self.Play Jump Sound` :!label _label_2))

(event `On Wall Jump`
  ;[1 1 1] SFX
  (goto _label_2))

(event `On Slide`
  ;[1 1 1] SFX
  (`GameplayStatics.PlaySoundAtLocation` "/Game/Audio/Movement/Slide2.Slide2" (`self.K2_GetActorLocation`) (struct) 1.0 (`KismetMathLibrary.RandomFloatInRange` 0.8 1.2) 0.0 "/Game/Audio/Movement/ATT_FootstepSound.ATT_FootstepSound" null null null))

(event `On Switch Weapon`
  ;[1 1 1] SFX
  (`self.Play Equip Sound`))

(event `On Muzzle Flash`
  (bind _muzzle_flash (`self.Muzzle Flash`))
  ;[1 1 1] Ranged Weapon
  (`ActorComponent.Activate` _muzzle_flash false)
  (`GameplayStatics.PlaySoundAtLocation` "/Game/Audio/Weapons/MusketFire2.MusketFire2" (`SceneComponent.K2_GetComponentLocation` _muzzle_flash) (struct) 1.0 1.0 0.0 "/Game/Audio/Weapons/ATT_MusketSound.ATT_MusketSound" null null null))

(fn `Bind To Base Events`
  (add `self.OnDeath` (`|CreateDelegate` :!event `On Death`))
  (add `self.OnAim` (`|CreateDelegate` :!event `On Aim`))
  (add `self.OnAimRelease` (`|CreateDelegate` :!event `On Aim Release`))
  (add `self.OnMuzzleFlash` (`|CreateDelegate` :!event `On Muzzle Flash`))
  (add `Weapon.OnActivate` (`self.RangedWeapon`) (`|CreateDelegate` :!event `On Ranged Weapon Activate`))
  (add `self.OnSlideJump` (`|CreateDelegate` :!event `On Slide Jump`))
  (add `self.OnWallJump` (`|CreateDelegate` :!event `On Wall Jump`))
  (add `self.OnLand` (`|CreateDelegate` :!event `On Land`))
  (add `self.OnSwitchWeapon` (`|CreateDelegate` :!event `On Switch Weapon`))
  (add `self.OnSlide` (`|CreateDelegate` :!event `On Slide`)))

(fn `Play Random Death Sound`
  (locals (`Death Sounds` :type "Array of SoundBase Object Reference"))
  (bind _death_sounds (`local.Death Sounds`))
  (`GameplayStatics.PlaySoundAtLocation` (`|GetArrayItem` _death_sounds (`KismetMathLibrary.RandomIntegerInRange` 0 (- (`KismetArrayLibrary.Array_Length` _death_sounds) 1))) (`self.K2_GetActorLocation`) (struct) 2.0 (`KismetMathLibrary.RandomFloatInRange` 0.9 1.1) 0.0 "/Game/Audio/Weapons/ATT_MusketSound.ATT_MusketSound" null null null))

(fn `UserConstructionScript`
  (add `self.OnHUDReady` (`|CreateDelegate` :!event `On HUD Ready`)))