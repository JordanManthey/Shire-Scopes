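; BP_ProjectileTrail is a projectile actor that carries a bullet trail effect forward at high speed.
; Tick counts frames up to a target delay, then a DoOnce activates the trail and sets the projectile movement's local forward velocity.
; An overlap deactivates the trail and destroys the actor after a short delay, with a BeginPlay timeout as the fallback lifetime.
; Hit events only print the other object's name.
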(event `self.ReceiveBeginPlay`
  (`KismetSystemLibrary.Delay` 5.0)
  (`self.K2_DestroyActor`))

(event `self.ReceiveTick`
  (params (DeltaSeconds :type "Float (single-precision)"))
  (if (>= (`self.Frame Count`) (`self.Target Frame Delay`))
    (`/Engine/EditorBlueprintResources/StandardMacros.DoOnce` false
      (:`Completed`
        (`ActorComponent.Activate` (`self.Bullet Trail`) false)
        (`ProjectileMovementComponent.SetVelocityInLocalSpace` (`self.ProjectileMovement`) (15000.0 0.0 0.0))))
    (else
      (`/Engine/EditorBlueprintResources/StandardMacros.IncrementInt` (`self.Frame Count`)))))

(event `self.ReceiveHit`
  (params (MyComp :type "PrimitiveComponent Object Reference") (Other :type "Actor Object Reference") (OtherComp :type "PrimitiveComponent Object Reference") (bSelfMoved :type Boolean) (HitLocation :type "Vector Structure") (HitNormal :type "Vector Structure") (NormalImpulse :type "Vector Structure") (Hit :type "HitResult Structure (by ref)"))
  (`KismetSystemLibrary.PrintString` (`KismetSystemLibrary.GetDisplayName` Other)))

(event `self.ReceiveActorBeginOverlap`
  (params (OtherActor :type "Actor Object Reference"))
  (`ActorComponent.Deactivate` (`self.Bullet Trail`))
  (`KismetSystemLibrary.Delay` 2.0)
  (`self.K2_DestroyActor`))

(fn `UserConstructionScript`)