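; Database manager that connects to a remote SQL database on BeginPlay to record and fetch the player win/loss leaderboard.
; UpdateLeaderboard sends batched queries built with FormatText, inserting missing players by SteamID, then incrementing winner and loser counts.
; RequestLeaderboardData selects rows ordered by wins, and successful results are rebroadcast through OnSelectQueryComplete.
; Connection credentials are hardcoded in the Blueprint, and player names go unescaped into the SQL.
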(event `self.OnConnectionStateChanged`
  (params (ConnectionStatus :type Boolean) (ConnectionID :type Integer) (ErrorMessage :type String))
  (if ConnectionStatus
    (set `self.Connection ID` ConnectionID)
    (`KismetSystemLibrary.PrintString` "CONNECTED TO DB" true true (struct :`R` 0.030624 :`G` 1.0 :`A` 1.0))
    (else
      (`KismetSystemLibrary.PrintString` "DB CONNECTION FAILED" true true (struct :`R` 1.0 :`A` 1.0)))))

(event `self.ReceiveBeginPlay`
  (`self.ConnectToDatabase`))

(event `self.OnQueryUpdateStatusChanged`
  (params (IsSuccessful :type Boolean) (ErrorMessage :type String))
  (if IsSuccessful
    (`KismetSystemLibrary.PrintString` "LEADERBOARD UPDATE SUCCESS" true true (struct :`R` 0.065589 :`G` 1.0 :`A` 1.0))
    (else
      (`KismetSystemLibrary.PrintString` "LEADERBOARD UPDATE FAILED" true true (struct :`R` 1.0 :`B` 0.038562 :`A` 1.0))
      (`KismetSystemLibrary.PrintString` ErrorMessage)
      (`KismetSystemLibrary.PrintString` (`self.Last Query`)))))

(event `self.ConnectToDatabase`
  (`self.CreateNewConnection` "aws.connect.psdb.cloud" "shire-scopes" "ta604faxsld6w0jcbyd0" "pscale_pw_jUxR83Om4TiRWzWldqLIfeuKK8npjT43ztaLpHs9l0E" (`|MakeMap` "")))

(event `self.OnQuerySelectStatusChanged`
  (params (IsSuccessful :type Boolean) (ErrorMessage :type String) (ResultByColumn :type "Array of MySQLDataTable Structure (by ref)") (ResultByRow :type "Array of MySQLDataRow Structure (by ref)"))
  (if IsSuccessful
    (`self.On Select Query Complete` ResultByRow)))

(event `self.UpdateLeaderboard`
  (params (WinningPlayerData :type "MatchPlayerData Structure") (LosingPlayerData :type "MatchPlayerData Structure"))
  (bind (_playername _playerid _steamid) (break `MatchPlayerData` WinningPlayerData))
  (bind (_playername_2 _playerid_2 _steamid_2) (break `MatchPlayerData` LosingPlayerData))
  (bind _returnvalue (`KismetTextLibrary.Conv_StringToText` _steamid))
  (bind _returnvalue_2 (`KismetTextLibrary.Conv_StringToText` _steamid_2))
  (bind _returnvalue_3 (`KismetTextLibrary.Conv_TextToString` (`|FormatText` "INSERT IGNORE INTO PlayerLeaderboard (PlayerID, PlayerName, WinCount, LossCount) VALUES({WinningPlayerID},\"{WinningPlayerName}\",0,0);" _returnvalue _playername)))
  (set `self.Last Query` _returnvalue_3)
  (`self.UpdateDataFromMultipleQueries` (`self.Connection ID`) (`|MakeArray` _returnvalue_3 (`KismetTextLibrary.Conv_TextToString` (`|FormatText` "UPDATE PlayerLeaderboard SET WinCount = WinCount + 1 WHERE PlayerID = {WinningPlayerID};" _returnvalue)) (`KismetTextLibrary.Conv_TextToString` (`|FormatText` "INSERT IGNORE INTO PlayerLeaderboard (PlayerID, PlayerName, WinCount, LossCount) VALUES({LosingPlayerID},\"{LosingPlayerName}\",0,0);" _returnvalue_2 _playername_2)) (`KismetTextLibrary.Conv_TextToString` (`|FormatText` "UPDATE PlayerLeaderboard SET LossCount = LossCount + 1 WHERE PlayerID = {LosingPlayerID};" _returnvalue_2)))))

(fn `Request Leaderboard Data`
  (`self.SelectDataFromQuery` (`self.Connection ID`) "SELECT * FROM PlayerLeaderboard ORDER BY WinCount DESC"))

(fn `UserConstructionScript`
  (`parent.UserConstructionScript`))