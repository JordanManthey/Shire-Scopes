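; Lobby player controller that creates the host or client lobby widget for the local player, based on authority.
; Local clients bind to game state lobby updates to refresh their widget, and ready changes are passed to the game state by player ID.
; Team caching writes to the game instance to allow hard travel, needing manual replication back to the server afterward.
; An unused PlayerState alternative, requiring seamless travel, remains in the graph.
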(event `self.ReceiveBeginPlay`
  (`self.Setup Lobby UI`)
  ;[1 1 1 1 14] Only Locally Controlled Clients need to be notified about Lobby updates. Server will update locally.
  (if (and (not (`self.HasAuthority`)) (`self.IsLocalController`))
    (add `LobbyGameState.OnLobbyUpdate` (`self.LobbyGameState`) (`|CreateDelegate` :!event `On Lobby Update`))))

(event `On Lobby Update`
  (bind _aswbp_lobby_client (cast `/Game/Blueprints/UI/Sessions/WBP_LobbyClient` (`self.Lobby UI`)))
  (`/Game/Blueprints/UI/Sessions/WBP_LobbyClient.On Lobby Update` _aswbp_lobby_client))

(event `On Ready Status Update`
  (params (NewReadyStatus :type Boolean))
  (`LobbyGameState.UpdateLobbyPlayerReadyStatus` (`self.LobbyGameState`) (`PlayerState.PlayerId` (`self.PlayerState`)) NewReadyStatus))

(fn `UserConstructionScript`)