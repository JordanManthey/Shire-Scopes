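; AI controller for Shire characters that runs the BT_ShireAI behavior tree from round start until death or round/match end.
; Sight and damage perception set the blackboard TargetPlayer, line-of-sight flag and focus, favoring enemies over damaged teammates.
; It also provides movement helpers with completion events: jump, slide-jump, velocity-preserving move abort, and a timeline yaw turn that temporarily overrides controller rotation.
; Stopping defers the tree shutdown one frame to avoid reset issues.
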(event `On Round/Match Over`
  (params (`Winning Team` :type Integer))
  (`self.Stop All Activity` :!label _label))

(event `On Round Start`
  (`self.StartBehavior`))

(event `On Death`
  (params (DeathCharacter :type "ShireCharacter Object Reference"))
  (goto _label))

(event `self.ReceiveBeginPlay`
  (bind _asbp_shire_game_state (cast `/Game/Blueprints/State/BP_ShireGameState` (`GameplayStatics.GetGameState`)))
  (add `ShireGameState.OnRoundOver` _asbp_shire_game_state (`|CreateDelegate` :!event `On Round/Match Over`))
  (add `ShireGameState.OnMatchOver` _asbp_shire_game_state (`|CreateDelegate` :!event `On Round/Match Over`)))

(event `self.StartBehavior`
  (`self.RunBehaviorTree` "/Game/AI/BT_ShireAI.BT_ShireAI")
  (`self.Setup Blackboard`))

(event `self.AI_Perception.OnTargetPerceptionUpdated`
  (params (Actor :type "Actor Object Reference") (Stimulus :type "AIStimulus Structure"))
  (`/Engine/EditorBlueprintResources/StandardMacros.IsValid` (`self.Blackboard`)
    (:`Is Valid`
      (`self.Handle Sight Sense` Actor Stimulus)
      (`self.Handle Damage Sense` Actor Stimulus))))

(event `self.ReceivePossess`
  (params (PossessedPawn :type "Pawn Object Reference"))
  (`self.Setup Character`)
  (add `ShireCharacter.OnDeath` (`self.Shire Character`) (`|CreateDelegate` :!event `On Death`))
  (bind _asbp_shire_game_state (cast `/Game/Blueprints/State/BP_ShireGameState` (`GameplayStatics.GetGameState`)))
  (add `ShireGameState.OnRoundStart` _asbp_shire_game_state (`|CreateDelegate` :!event `On Round Start`)))

(event `Lerp Rotate Character`
  (params (`Target Rotator` :type "Rotator Structure") (`Override Controller Rotation On Finish` :type Boolean :default false))
  (`self.Override Character Rotation Control`)
  (`self.Set Rotation Vars` `Target Rotator`)
  (`self.Setup Rotation Lerp Rate`)
  (bind (_direction _lerp_alpha) (`Timeline|Lerp Rotate Character Timeline` :!via `PlayFromStart`)
    (:`Update`
      (`self.Update Character Rotation` _lerp_alpha))
    (:`Finished`
      (if (not `Override Controller Rotation On Finish`)
        (`self.Release Character Rotation Control`))
      (`self.Lerp Rotate Character Finished`))))

(event `AI SlideJump`
  (`self.AI Slide Executed`) ; Must broadcast before slide so AI movement no longer overrides.
  (`ShireCharacter.UseSlideAbility` (`self.Shire Character`))
  (`KismetSystemLibrary.Delay` (`KismetMathLibrary.RandomFloatInRange` 0.25 0.5))
  (`Character.Jump` (`self.Shire Character`))
  (`self.AI SlideJump Executed`))

(fn `Abort AI MoveTo`
  (params (`Maintain Velocity` :type Boolean :default true))
  (locals (`Cached Velocity` :type "Vector Structure"))
  (bind _charactermovement (`Character.CharacterMovement` (`self.Shire Character`)))
  (set `local.Cached Velocity` (`MovementComponent.Velocity` _charactermovement))
  (`MovementComponent.StopMovementImmediately` _charactermovement)
  (if `Maintain Velocity`
    (set `MovementComponent.Velocity` (`local.Cached Velocity`) _charactermovement)))

(fn `AI Jump`
  (`Character.Jump` (`self.Shire Character`))
  (`self.AI Jump Executed`))

(fn `Handle Damage Sense`
  (params (Actor :type "Actor Object Reference") (Stimulus :type "AIStimulus Structure"))
  (locals (`Seen Shire Character` :type "/Game/Blueprints/Actors/BP_ShireCharacter Object Reference"))
  (bind _returnvalue (`AIPerceptionSystem.GetSenseClassForStimulus` Stimulus))
  (if (== _returnvalue "/Script/AIModule.AISense_Damage")
    (`/Engine/EditorBlueprintResources/StandardMacros.IsValid` (`BlackboardComponent.GetValueAsObject` (`self.Blackboard`) "TargetPlayer") ; Only assign target if no TargetPlayer exists OR if current TargetPlayer is teammate.
      (:`Is Valid`
        (bind _asbp_shire_character (cast `/Game/Blueprints/Actors/BP_ShireCharacter` (`BlackboardComponent.GetValueAsObject` (`self.Blackboard`) "TargetPlayer")))
        (bind _returnvalue_2 (`ShireCharacter.IsTeammate` _asbp_shire_character (`self.Shire Character`)))
        (if _returnvalue_2
          (`BlackboardComponent.SetValueAsObject` (`self.Blackboard`) "TargetPlayer" (`local.Actor`) :!label _label)))
      (:`Is Not Valid`
        (goto _label)))))

(fn `Handle Sight Sense`
  (params (Actor :type "Actor Object Reference") (Stimulus :type "AIStimulus Structure"))
  (locals (`Seen Shire Character` :type "/Game/Blueprints/Actors/BP_ShireCharacter Object Reference"))
  (bind _seen_shire_character (`local.Seen Shire Character`))
  (bind _returnvalue (`BlackboardComponent.GetValueAsObject` (`self.Blackboard`) "TargetPlayer"))
  (bind _returnvalue_2 (`AIPerceptionSystem.GetSenseClassForStimulus` Stimulus))
  (if (== _returnvalue_2 "/Script/AIModule.AISense_Sight")
    (bind _info (`AIPerceptionComponent.GetActorsPerception` (`self.GetAIPerceptionComponent`) (`local.Actor`)))
    (if (`.bSuccessfullySensed` (break `AIStimulus` (`|GetArrayItem` (`.LastSensedStimuli` (break `ActorPerceptionBlueprintInfo` _info)))))
      (bind _asbp_shire_character (cast `/Game/Blueprints/Actors/BP_ShireCharacter` (`local.Actor`)))
      (bind _output_get (set `local.Seen Shire Character` _asbp_shire_character))
      (bind _returnvalue_3 (`ShireCharacter.IsDead` _output_get))
      (if (not _returnvalue_3)
        (bind _returnvalue_4 (`ShireCharacter.IsTeammate` _output_get (`self.Shire Character`)))
        (if _returnvalue_4
          ;[1 1 1] If the seen character is a damaged teammate and we don't already have a target.
          (`/Engine/EditorBlueprintResources/StandardMacros.IsValid` (`BlackboardComponent.GetValueAsObject` (`self.Blackboard`) "TargetPlayer")
            (:`Is Not Valid`
              (if (< (`ShireCharacter.Health` _seen_shire_character) (`ShireCharacter.MaxHealth` _seen_shire_character))
                (`BlackboardComponent.SetValueAsObject` (`self.Blackboard`) "TargetPlayer" (`local.Seen Shire Character`))
                (`BlackboardComponent.SetValueAsBool` (`self.Blackboard`) "HasTargetLOS" true)
                (`self.K2_SetFocus` (`local.Seen Shire Character`)))))
          (else
            (`/Engine/EditorBlueprintResources/StandardMacros.IsValid` (`BlackboardComponent.GetValueAsObject` (`self.Blackboard`) "TargetPlayer")
              (:`Is Valid`
                ;[1 1 1] If the seen character is our current target, or the seen character is an enemy and our current target is a teammate --> focus the seen character.
                (bind _asbp_shire_character_2 (cast `/Game/Blueprints/Actors/BP_ShireCharacter` _returnvalue))
                (bind _returnvalue_5 (`ShireCharacter.IsTeammate` _asbp_shire_character_2 (`self.Shire Character`)))
                (if (or _returnvalue_5 (== (`local.Actor`) _returnvalue))
                  (`BlackboardComponent.SetValueAsObject` (`self.Blackboard`) "TargetPlayer" (`local.Seen Shire Character`))
                  (`BlackboardComponent.SetValueAsBool` (`self.Blackboard`) "HasTargetLOS" true)
                  (`self.K2_SetFocus` (`local.Seen Shire Character`))))
              (:`Is Not Valid`
                ;[1 1 1] If the seen character is an enemy and we don't already have a target.
                (`BlackboardComponent.SetValueAsObject` (`self.Blackboard`) "TargetPlayer" (`local.Seen Shire Character`))
                (`BlackboardComponent.SetValueAsBool` (`self.Blackboard`) "HasTargetLOS" true)
                (`self.K2_SetFocus` (`local.Seen Shire Character`)))))))
      (else
        ;[1 1 1 1 14] If the character leaving sight is the current TargetPlayer, set HasTargetLOS to false.
        (if (== (`local.Actor`) (`BlackboardComponent.GetValueAsObject` (`self.Blackboard`) "TargetPlayer"))
          (`BlackboardComponent.SetValueAsBool` (`self.Blackboard`) "HasTargetLOS" false)
          (`self.K2_ClearFocus`))))))

(fn `Update Visited Locations`
  (params (`New Location` :type "Vector Structure"))
  (bind _recent_visited_locations (`self.Recent Visited Locations`))
  (if (>= (`KismetArrayLibrary.Array_Length` (`self.Recent Visited Locations`)) 3)
    (`KismetArrayLibrary.Array_Remove` _recent_visited_locations))
  (`KismetArrayLibrary.Array_Add` _recent_visited_locations (`local.New Location`)))

(fn `UserConstructionScript`)